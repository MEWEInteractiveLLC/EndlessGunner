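; Orb pickup for a runner game that counts as a coin and appears to represent dark matter.
; When the third-person character overlaps its sphere, it calls AddCoins on the game mode and plays an impact sound at the item's location.
; It then triggers the player character's dark matter pickup tutorial on every pickup and destroys itself.
; A DoOnce node in the graph is unconnected and never runs.
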(event OnComponentBeginOverlap(Sphere)
  (params (OverlappedComponent :type Primitive%20Component%20Object%20Reference) (OtherActor :type Actor%20Object%20Reference) (OtherComp :type Primitive%20Component%20Object%20Reference) (OtherBodyIndex :type Integer) (bFromSweep :type Boolean) (SweepResult :type Hit%20Result%20Structure%20%28by%20ref%29))
  (Utilities|Casting|CastToThirdPersonCharacter OtherActor)
  (Utilities|Casting|CastToThirdPersonGameMode (Game|GetGameMode))
  (bind _asthird_person_game_mode (Utilities|Casting|CastToThirdPersonGameMode (Game|GetGameMode)))
  (Default|AddCoins _asthird_person_game_mode)
  (Audio|PlaySoundatLocation "/Game/SciFiWeapLight/Sound/Rifle/Wavs/Rifle_ImpactBody06.Rifle_ImpactBody06" (Transformation|GetWorldLocation (Variables|Default|GetItem)) "0, 0, 0" 0.65 0.8 0.0 0 0 0)
  (bind _asthird_person_character (Utilities|Casting|CastToThirdPersonCharacter (Game|GetPlayerCharacter 0)))
  (Default|DarkMatterPickUpTutorial _asthird_person_character)
  (Actor|DestroyActor))

(event EventBeginPlay
  (|CallParentFunction) ; This node is disabled and will not be called.\nDrag off pins to build functionality.
)

(event Collision|EventActorBeginOverlap
  (params (OtherActor :type Actor%20Object%20Reference))
  (|CallParentFunction OtherActor) ; This node is disabled and will not be called.\nDrag off pins to build functionality.
)

(event EventTick
  (params (DeltaSeconds :type Float%20%28single-precision%29))
  (|CallParentFunction DeltaSeconds) ; This node is disabled and will not be called.\nDrag off pins to build functionality.
)

(fn ConstructionScript
  (|CallParentFunction))