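; Ammo pickup actor that resupplies the player character's spare ammo when touched.
; A Sphere overlap casts to ThirdPersonCharacter and, if spare ammo is below max, calls GiveAmmo with a random count between a fixed minimum and Amount, then plays a sound.
; At full ammo it only prints a message.
; The graph never destroys or disables the pickup.
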(event OnComponentBeginOverlap(Sphere)
  (params (OverlappedComponent :type Primitive%20Component%20Object%20Reference) (OtherActor :type Actor%20Object%20Reference) (OtherComp :type Primitive%20Component%20Object%20Reference) (OtherBodyIndex :type Integer) (bFromSweep :type Boolean) (SweepResult :type Hit%20Result%20Structure%20%28by%20ref%29))
  (bind _asthird_person_character (Utilities|Casting|CastToThirdPersonCharacter OtherActor))
  (if (< (Variables|/Game/ThirdPersonBP/Blueprints/ThirdPersonCharacter.ThirdPersonCharacter_C|GetCurrentSpareAmmo _asthird_person_character) (Variables|/Game/ThirdPersonBP/Blueprints/ThirdPersonCharacter.ThirdPersonCharacter_C|GetMaxAmmo _asthird_person_character))
    (Default|GiveAmmo _asthird_person_character (Math|Random|RandomIntegerinRange 8 (Variables|Default|GetAmount)))
    (Audio|PlaySoundatLocation 0 (Transformation|GetActorLocation _asthird_person_character) "0, 0, 0" 1.0 1.0 0.0 0 0 0)
    (else
      (Development|PrintString "Ammo Full"))))

(event EventBeginPlay
  (|CallParentFunction) ; This node is disabled and will not be called.\nDrag off pins to build functionality.
)

(event Collision|EventActorBeginOverlap
  (params (OtherActor :type Actor%20Object%20Reference))
  (|CallParentFunction OtherActor) ; This node is disabled and will not be called.\nDrag off pins to build functionality.
)

(event EventTick
  (params (DeltaSeconds :type Float%20%28single-precision%29))
  (|CallParentFunction DeltaSeconds) ; This node is disabled and will not be called.\nDrag off pins to build functionality.
)

(fn ConstructionScript
  (|CallParentFunction))