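; BP_ChaserEnemy is a suicide enemy that chases the player and explodes on contact.
; Pawn sensing starts an AI MoveTo toward a seen ThirdPersonCharacter, and a capsule hit on one calls DamagePlayer.
; DamagePlayer damages player 0, plays explosion sound and particles, then destroys the enemy.
; BlowUp, not called here, is a smaller, quieter explosion that increments the game mode's EnemiesKilled before destroying the enemy.
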(event OnSeePawn(PawnSensing)
  (params (Pawn :type Pawn%20Object%20Reference))
  (bind _asthird_person_character (Utilities|Casting|CastToThirdPersonCharacter Pawn))
  (AI|AIMoveTo self "0, 0, 0" _asthird_person_character 5.0 false))

(event OnComponentHit(CapsuleComponent)
  (params (HitComponent :type Primitive%20Component%20Object%20Reference) (OtherActor :type Actor%20Object%20Reference) (OtherComp :type Primitive%20Component%20Object%20Reference) (NormalImpulse :type Vector :default "0, 0, 0") (Hit :type Hit%20Result%20Structure%20%28by%20ref%29))
  (Utilities|Casting|CastToThirdPersonCharacter OtherActor)
  (CallFunction|DamagePlayer))

(fn ConstructionScript)

(fn DamagePlayer
  (bind _mesh (Variables|Character|GetMesh))
  (bind _returnvalue (Transformation|GetWorldLocation _mesh))
  (bind _asthird_person_character (Utilities|Casting|CastToThirdPersonCharacter (Game|GetPlayerCharacter 0)))
  (Game|Damage|ApplyDamage _asthird_person_character (Variables|Default|GetDamage) 0 self "/Script/Engine.DamageType")
  ;[1 1 1] Blow Up
  (Audio|PlaySoundatLocation "/Game/SciFiWeapLight/Sound/GrenadeLauncher/Wavs/GL_Explosion02.GL_Explosion02" _returnvalue "0, 0, 0" 0.65 1.0 0.0 0 0 0)
  (Effects|SpawnEmitteratLocation "/Game/SciFiWeapLight/FX/Particles/P_Grenade_Explosion_Dark.P_Grenade_Explosion_Dark" _returnvalue)
  (Actor|SetLifeSpan 0.75)
  (Actor|DestroyActor))

(fn BlowUp
  (bind _mesh (Variables|Character|GetMesh))
  (bind _returnvalue (Transformation|GetWorldLocation _mesh))
  (Audio|PlaySoundatLocation "/Game/SciFiWeapLight/Sound/GrenadeLauncher/Wavs/GL_Explosion02.GL_Explosion02" _returnvalue "0, 0, 0" 0.4 1.0 0.0 0 0 0)
  (Effects|SpawnEmitteratLocation "/Game/SciFiWeapLight/FX/Particles/P_Grenade_Explosion_Dark.P_Grenade_Explosion_Dark" _returnvalue "0, 0, 0" "0.100000,0.100000,0.100000")
  (bind _asthird_person_game_mode (Utilities|Casting|CastToThirdPersonGameMode (Game|GetGameMode)))
  (bind _result (Math|Integer|IncrementInt (Variables|/Game/ThirdPersonBP/Blueprints/ThirdPersonGameMode.ThirdPersonGameMode_C|GetEnemiesKilled _asthird_person_game_mode))
    (:%20%20
      (Variables|/Game/ThirdPersonBP/Blueprints/ThirdPersonGameMode.ThirdPersonGameMode_C|SetEnemiesKilled _asthird_person_game_mode _result)
      (Actor|SetLifeSpan 0.75)
      (Actor|DestroyActor))))