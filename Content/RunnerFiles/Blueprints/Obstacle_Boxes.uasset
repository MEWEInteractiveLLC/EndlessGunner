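; Box obstacle for a runner game that explodes when the third-person character hits it.
; On component hit it applies damage to the character unless dash mode is active.
; Either way it plays an explosion sound, spawns an explosion emitter and destroys itself.
; The delayed emitter cleanup is wired after DestroyActor, so it depends on an actor already being destroyed.
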(event OnComponentHit(Obstacle)
  (params (HitComponent :type Primitive%20Component%20Object%20Reference) (OtherActor :type Actor%20Object%20Reference) (OtherComp :type Primitive%20Component%20Object%20Reference) (NormalImpulse :type Vector :default "0, 0, 0") (Hit :type Hit%20Result%20Structure%20%28by%20ref%29))
  (bind _obstacle (Variables|Default|GetObstacle))
  (bind _returnvalue (Transformation|GetWorldLocation _obstacle))
  ;[1 1 1] Comment
  (bind _asthird_person_character (Utilities|Casting|CastToThirdPersonCharacter OtherActor))
  (if (Variables|/Game/ThirdPersonBP/Blueprints/ThirdPersonCharacter.ThirdPersonCharacter_C|GetisDashModeActive _asthird_person_character)
    (Audio|PlaySoundatLocation "/Game/MobileStarterContent/Audio/Explosion01.Explosion01" _returnvalue "0, 0, 0" 1.0 1.0 0.0 0 0 0)
    (else
      (Audio|PlaySoundatLocation "/Game/MobileStarterContent/Audio/Explosion01.Explosion01" _returnvalue "0, 0, 0" 1.0 1.0 0.0 0 0 0)
      (Game|Damage|ApplyDamage _asthird_person_character (Variables|Default|GetDamageAmount) 0 self "/Script/Engine.DamageType")))
  (bind _returnvalue_2 (Effects|SpawnEmitteratLocation "/Game/MobileStarterContent/Particles/P_Explosion.P_Explosion" _returnvalue))
  (Actor|DestroyActor)
  (Utilities|FlowControl|Delay 0.5)
  (Components|DestroyComponent _returnvalue_2))

(event EventBeginPlay
  (|CallParentFunction) ; This node is disabled and will not be called.\nDrag off pins to build functionality.
)

(event Collision|EventActorBeginOverlap
  (params (OtherActor :type Actor%20Object%20Reference))
  (|CallParentFunction OtherActor) ; This node is disabled and will not be called.\nDrag off pins to build functionality.
)

(event EventTick
  (params (DeltaSeconds :type Float%20%28single-precision%29))
  (|CallParentFunction DeltaSeconds) ; This node is disabled and will not be called.\nDrag off pins to build functionality.
)

(fn ConstructionScript
  (|CallParentFunction))