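; Base floor tile for an endless runner that fills its three lanes with random obstacles and coins on BeginPlay.
; Pipe or box obstacles and coins roll independently, each in a nested chain where a lane can spawn only if the previous one did.
; When the character overlaps the box trigger, the tile has the game mode spawn tiles, adds multiplied points, raises clamped walk speed, then destroys itself after a delay.
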(event OnComponentBeginOverlap(Box)
  (params (OverlappedComponent :type Primitive%20Component%20Object%20Reference) (OtherActor :type Actor%20Object%20Reference) (OtherComp :type Primitive%20Component%20Object%20Reference) (OtherBodyIndex :type Integer) (bFromSweep :type Boolean) (SweepResult :type Hit%20Result%20Structure%20%28by%20ref%29))
  (Utilities|Casting|CastToThirdPersonCharacter OtherActor)
  (bind _asthird_person_game_mode (Utilities|Casting|CastToThirdPersonGameMode (Game|GetGameMode)))
  (Default|SpawnTiles _asthird_person_game_mode)
  (bind _asthird_person_game_mode_2 (Utilities|Casting|CastToThirdPersonGameMode (Game|GetGameMode)))
  (Variables|/Game/ThirdPersonBP/Blueprints/ThirdPersonGameMode.ThirdPersonGameMode_C|SetCurrentPoints _asthird_person_game_mode_2 (+ (Variables|/Game/ThirdPersonBP/Blueprints/ThirdPersonGameMode.ThirdPersonGameMode_C|GetCurrentPoints _asthird_person_game_mode_2) (* 1 (Variables|/Game/ThirdPersonBP/Blueprints/ThirdPersonGameMode.ThirdPersonGameMode_C|GetPointsMultiplier _asthird_person_game_mode_2))))
  (bind _asthird_person_character (Utilities|Casting|CastToThirdPersonCharacter (Game|GetPlayerCharacter 0)))
  (Variables|/Script/Engine.CharacterMovementComponent|SetMaxWalkSpeed (Variables|/Script/Engine.Character|GetCharacterMovement _asthird_person_character) (Math|Float|Clamp(Float) (* (Variables|/Script/Engine.CharacterMovementComponent|GetMaxWalkSpeed (Variables|/Script/Engine.Character|GetCharacterMovement _asthird_person_character)) 1.0075) 6e+02 2.5e+03))
  (Utilities|FlowControl|Delay 1.0)
  (Actor|DestroyActor))

(event EventBeginPlay
  (CallFunction|SpawnObstacles)
  (CallFunction|SpawnPickups))

(event Collision|EventActorBeginOverlap
  (params (OtherActor :type Actor%20Object%20Reference)))

(event EventTick
  (params (DeltaSeconds :type Float%20%28single-precision%29)))

(fn ConstructionScript)

(fn SpawnObstacles
  (bind _lane2 (Variables|Default|GetLane2))
  (bind _lane0 (Variables|Default|GetLane0))
  (bind _lane1 (Variables|Default|GetLane1))
  (bind _returnvalue (Transformation|GetWorldTransform _lane2))
  (bind _returnvalue_2 (Transformation|GetWorldTransform _lane1))
  (bind _returnvalue_3 (Transformation|GetWorldTransform _lane0))
  (Utilities|IsValid (Variables|Default|GetObstacles)
    (:Is%20Not%20Valid
      ;[1 1 1] Spawns In the LOW PIPE OBSTACLE
      (switch int (Math|Random|RandomIntegerinRange 0 4)
        (:1
          (Game|SpawnActorfromClass "/Game/RunnerFiles/Blueprints/Obstacle_Pipes.Obstacle_Pipes_C" (Math|Transform|MakeTransform (.location _returnvalue_3) "0, 0, 0" "1,1,1") "Undefined" 0 0))
        (:2
          ;[1 1 1] Spawns In the Box At Random
          (Game|SpawnActorfromClass "/Game/RunnerFiles/Blueprints/Obstacle_Boxes.Obstacle_Boxes_C" (Math|Transform|MakeTransform (.location _returnvalue_3) "0, 0, 0" "1,1,1") "Undefined" 0 0)))
      (switch int (Math|Random|RandomIntegerinRange 0 3)
        (:1
          (Game|SpawnActorfromClass "/Game/RunnerFiles/Blueprints/Obstacle_Pipes.Obstacle_Pipes_C" (Math|Transform|MakeTransform (.location _returnvalue_2) "0, 0, 0" "1,1,1") "Undefined" 0 0))
        (:2
          (Game|SpawnActorfromClass "/Game/RunnerFiles/Blueprints/Obstacle_Boxes.Obstacle_Boxes_C" (Math|Transform|MakeTransform (.location _returnvalue_2) "0, 0, 0" "1,1,1") "Undefined" 0 0)))
      (switch int (Math|Random|RandomIntegerinRange 0 3)
        (:1
          (Game|SpawnActorfromClass "/Game/RunnerFiles/Blueprints/Obstacle_Pipes.Obstacle_Pipes_C" (Math|Transform|MakeTransform (.location _returnvalue) "0, 0, 0" "1,1,1") "Undefined" 0 0))
        (:2
          (Game|SpawnActorfromClass "/Game/RunnerFiles/Blueprints/Obstacle_Boxes.Obstacle_Boxes_C" (Math|Transform|MakeTransform (.location _returnvalue) "0, 0, 0" "1,1,1") "Undefined" 0 0))))))

(fn SpawnPickups
  ;[1 1 1] Spawns Coin Pickups
  (switch int (Math|Random|RandomIntegerinRange 0 3)
    (:1
      (Game|SpawnActorfromClass "/Game/RunnerFiles/Blueprints/Pickup_Coin.Pickup_Coin_C" (Math|Transform|MakeTransform (.location (Transformation|GetWorldTransform (Variables|Default|GetLane0))) "0, 0, 0" "1,1,1") "Undefined" 0 0)
      (switch int (Math|Random|RandomIntegerinRange 0 3)
        (:1
          (Game|SpawnActorfromClass "/Game/RunnerFiles/Blueprints/Pickup_Coin.Pickup_Coin_C" (Math|Transform|MakeTransform (.location (Transformation|GetWorldTransform (Variables|Default|GetLane1))) "0, 0, 0" "1,1,1") "Undefined" 0 0)
          (switch int (Math|Random|RandomIntegerinRange 0 3)
            (:1
              (Game|SpawnActorfromClass "/Game/RunnerFiles/Blueprints/Pickup_Coin.Pickup_Coin_C" (Math|Transform|MakeTransform (.location (Transformation|GetWorldTransform (Variables|Default|GetLane2))) "0, 0, 0" "1,1,1") "Undefined" 0 0))))))))