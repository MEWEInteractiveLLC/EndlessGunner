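; Pipe obstacle actor for the runner game that kills the third-person character on overlap unless dash mode is active.
; A dashing hit disables the obstacle's collision and plays a sound.
; Otherwise it calls the player's death, clears widgets, shows the mouse cursor, plays a sound and displays the GameOverScreen widget.
; The obstacle destroys itself after either outcome.
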(event OnComponentBeginOverlap(Obstacle)
  (params (OverlappedComponent :type Primitive%20Component%20Object%20Reference) (OtherActor :type Actor%20Object%20Reference) (OtherComp :type Primitive%20Component%20Object%20Reference) (OtherBodyIndex :type Integer) (bFromSweep :type Boolean) (SweepResult :type Hit%20Result%20Structure%20%28by%20ref%29))
  ;[1 1 1] Collision Kills Player and pops up a game over screen
  (bind _asthird_person_character (Utilities|Casting|CastToThirdPersonCharacter OtherActor))
  (if (Variables|/Game/ThirdPersonBP/Blueprints/ThirdPersonCharacter.ThirdPersonCharacter_C|GetisDashModeActive _asthird_person_character)
    (Collision|SetCollisionEnabled (Variables|Default|GetObstacle) "NoCollision")
    (Audio|PlaySoundatLocation 0 "0, 0, 0" "0, 0, 0" 1.0 1.0 0.0 0 0 0)
    (else
      (Default|PlayerDeath _asthird_person_character)
      (Viewport|RemoveAllWidgets)
      (Variables|/Script/Engine.PlayerController|SetbShowMouseCursor (Game|GetPlayerController 0) true)
      (Audio|PlaySoundatLocation 0 "0, 0, 0" "0, 0, 0" 1.0 1.0 0.0 0 0 0)
      (bind _returnvalue (UserInterface|CreateWidget "/Game/RunnerFiles/UI_ELEMENTS/GameOverScreen.GameOverScreen_C"))
      (UserInterface|Viewport|AddtoViewport _returnvalue 0)))
  (Actor|DestroyActor))

(event EventBeginPlay
  (|CallParentFunction) ; This node is disabled and will not be called.\nDrag off pins to build functionality.
)

(event Collision|EventActorBeginOverlap
  (params (OtherActor :type Actor%20Object%20Reference))
  (|CallParentFunction OtherActor) ; This node is disabled and will not be called.\nDrag off pins to build functionality.
)

(event EventTick
  (params (DeltaSeconds :type Float%20%28single-precision%29))
  (|CallParentFunction DeltaSeconds) ; This node is disabled and will not be called.\nDrag off pins to build functionality.
)

(fn ConstructionScript
  (|CallParentFunction))