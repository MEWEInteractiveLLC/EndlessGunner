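; Ammo pickup actor that gives ammo to the player character on touch.
; When its Box begins overlapping a ThirdPersonCharacter, it calls GiveAmmo with its Amount variable.
; It then spawns a muzzle-flash particle effect at the Item component's location and destroys itself, with no respawn.
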(event OnComponentHit(Box)
  (params (HitComponent :type Primitive%20Component%20Object%20Reference) (OtherActor :type Actor%20Object%20Reference) (OtherComp :type Primitive%20Component%20Object%20Reference) (NormalImpulse :type Vector :default "0, 0, 0") (Hit :type Hit%20Result%20Structure%20%28by%20ref%29)))

(event OnComponentBeginOverlap(Box)
  (params (OverlappedComponent :type Primitive%20Component%20Object%20Reference) (OtherActor :type Actor%20Object%20Reference) (OtherComp :type Primitive%20Component%20Object%20Reference) (OtherBodyIndex :type Integer) (bFromSweep :type Boolean) (SweepResult :type Hit%20Result%20Structure%20%28by%20ref%29))
  (bind _asthird_person_character (Utilities|Casting|CastToThirdPersonCharacter OtherActor))
  (Default|GiveAmmo _asthird_person_character (Variables|Default|GetAmount))
  (Effects|SpawnEmitteratLocation "/Game/SciFiWeapLight/FX/Particles/P_Shotgun_MuzzleFlash_Light.P_Shotgun_MuzzleFlash_Light" (Transformation|GetWorldLocation (Variables|Default|GetItem)) "0, 0, 0" "1.300000,1.300000,1.300000")
  (Actor|DestroyActor))

(event EventBeginPlay
  (|CallParentFunction) ; This node is disabled and will not be called.\nDrag off pins to build functionality.
)

(event Collision|EventActorBeginOverlap
  (params (OtherActor :type Actor%20Object%20Reference))
  (|CallParentFunction OtherActor) ; This node is disabled and will not be called.\nDrag off pins to build functionality.
)

(event EventTick
  (params (DeltaSeconds :type Float%20%28single-precision%29))
  (|CallParentFunction DeltaSeconds) ; This node is disabled and will not be called.\nDrag off pins to build functionality.
)

(fn ConstructionScript
  (|CallParentFunction))