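; Collectible coin pickup for the runner game.
; When the third-person character overlaps its sphere, it tells the third-person game mode to add coins, plays a pickup sound at the item's location and destroys itself.
; All logic lives in the sphere overlap event; the default BeginPlay, overlap and Tick events are unused.
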(event OnComponentBeginOverlap(Sphere)
  (params (OverlappedComponent :type Primitive%20Component%20Object%20Reference) (OtherActor :type Actor%20Object%20Reference) (OtherComp :type Primitive%20Component%20Object%20Reference) (OtherBodyIndex :type Integer) (bFromSweep :type Boolean) (SweepResult :type Hit%20Result%20Structure%20%28by%20ref%29))
  (Utilities|Casting|CastToThirdPersonCharacter OtherActor)
  (Utilities|Casting|CastToThirdPersonGameMode (Game|GetGameMode))
  (bind _asthird_person_game_mode (Utilities|Casting|CastToThirdPersonGameMode (Game|GetGameMode)))
  (Default|AddCoins _asthird_person_game_mode)
  (Audio|PlaySoundatLocation "/Game/RunnerFiles/SFX/Pickup_SFX.Pickup_SFX" (Transformation|GetWorldLocation (Variables|Default|GetItem)) "0, 0, 0" 1.0 1.0 0.0 0 0 0)
  (Actor|DestroyActor))

(event EventBeginPlay
  (|CallParentFunction) ; This node is disabled and will not be called.\nDrag off pins to build functionality.
)

(event Collision|EventActorBeginOverlap
  (params (OtherActor :type Actor%20Object%20Reference))
  (|CallParentFunction OtherActor) ; This node is disabled and will not be called.\nDrag off pins to build functionality.
)

(event EventTick
  (params (DeltaSeconds :type Float%20%28single-precision%29))
  (|CallParentFunction DeltaSeconds) ; This node is disabled and will not be called.\nDrag off pins to build functionality.
)

(fn ConstructionScript
  (|CallParentFunction))